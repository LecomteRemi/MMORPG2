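; Patrol route actor for enemy AI that supplies waypoints from the points of a PatrolRoute spline.
; GetSplinePointAsWorldPosition returns the world location of the spline point at the current PatrolIndex.
; The incrementpatrolroute event advances that index, wrapping around when Loop is set.
; Otherwise it ping-pongs, flipping Direction when the index equals the point count (one past the last point) or zero.
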(event `increment patrol route`
  (if (`self.Loop`)
    (set `self.PatrolIndex` (mod (+ (`self.PatrolIndex`) 1) (`SplineComponent.GetNumberOfSplinePoints` (`self.patrol_route`))))
    (else
      (bind _output_get (set `self.PatrolIndex` (+ (`self.PatrolIndex`) (`self.Direction`))))
      (if (== _output_get (`SplineComponent.GetNumberOfSplinePoints` (`self.patrol_route`)))
        (set `self.Direction` -1)
        (elif (== _output_get 0)
          (set `self.Direction` 1))))))

(fn `getSplinePointAsWorldPosition`
  (returns (position :type "Vector Structure"))
  (return (`SplineComponent.GetLocationAtSplinePoint` (`self.patrol_route`) (`self.PatrolIndex`) "World")))

(fn `UserConstructionScript`)