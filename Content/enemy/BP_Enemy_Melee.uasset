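; BP_Enemy_Melee is a sword-wielding enemy child Blueprint that sets its type to SwordsMan and implements attack, equip and unequip behavior.
; Montage notifies time the weapon spawn and hand-socket attach, its destruction, and a forward sphere trace that sends damage to a hit pawn.
; Attacks block interruption until the montage ends, and completion calls notify listeners.
; SetMovementSpeed maps movement states to walk speeds.
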(event `self.ReceiveBeginPlay`
  (`parent.ReceiveBeginPlay`)
  (set `self.EnemyType` "SwordsMan"))

(event `/Game/enemy/AI/BPI_EnemyAI.Attack`
  (bind _returnvalue (`self.K2_GetActorLocation`))
  (bind _bpc_damagesystem (`self.BPC_DamageSystem`))
  (bind _notifyname (`|PlayMontage` (`self.Mesh`) "/Game/Characters/Mannequins/Animations/SwordAnims/sword_slash.sword_slash")
    (:`then`
      (set `/Game/DamageSystem/BPC_DamageSystem.isInterruptible` false _bpc_damagesystem))
    (:`OnCompleted`
      (set `/Game/DamageSystem/BPC_DamageSystem.isInterruptible` true _bpc_damagesystem :!label _label)
      (`self.On attack end`))
    (:`OnInterrupted`
      (goto _label))
    (:`OnNotifyBegin`
      (switch `name` _notifyname
        (:`Slash`
          (bind (_outhit _returnvalue_2) (`KismetSystemLibrary.SphereTraceSingleForObjects` :`Start` _returnvalue :`End` (+ _returnvalue (* (`self.GetActorForwardVector`) 200.0)) :`Radius` 20.0 :`ObjectTypes` (`|MakeArray` "ObjectTypeQuery3" :!type "EObjectTypeQuery Enum") :`DrawDebugType` "ForDuration"))
          (if _returnvalue_2
            (message `/Game/DamageSystem/BPI_Damageable.TakeDamage` (`.HitActor` (`GameplayStatics.BreakHitResult` _outhit)) (make `/Game/DamageSystem/S_DamageInfo` 20.0 "NewEnumerator1" "NewEnumerator2") self)))))))

(event `/Game/enemy/AI/BPI_EnemyAI.EquipWeapon`
  (bind _notifyname (`|PlayMontage` (`self.Mesh`) "/Game/Characters/Mannequins/Animations/SwordAnims/Unsheathing_Montage.Unsheathing_Montage")
    (:`OnCompleted`
      (`self.On weapon equiped`))
    (:`OnNotifyBegin`
      (switch `name` _notifyname
        (:`GrabSword`
          (bind _returnvalue (`|SpawnActorFromClass` "/Game/weapons/blueprints/BP_WeaponSword.BP_WeaponSword_C" (`self.GetTransform`) "Undefined" "MultiplyWithRoot" null null))
          (bind _output_get (set `self.WeaponActor` _returnvalue))
          (`self.K2_AttachToComponent` _output_get (`self.Mesh`) "hand_rSocket" "SnapToTarget" "SnapToTarget" "SnapToTarget" true)
          (set `self.is_weilding_weapon` true))))))

(event `/Game/enemy/AI/BPI_EnemyAI.UnequipWeapon`
  (bind _notifyname (`|PlayMontage` (`self.Mesh`) "/Game/Characters/Mannequins/Animations/SwordAnims/SheathingSword_UE_Montage.SheathingSword_UE_Montage")
    (:`OnCompleted`
      (`self.On weapon unequiped`))
    (:`OnNotifyBegin`
      (switch `name` _notifyname
        (:`DropSword`
          (`self.K2_DestroyActor` (`self.WeaponActor`))
          (set `self.is_weilding_weapon` false))))))

(fn `SetMovementSpeed`
  (params (Speed :type "/Game/enemy/AI/Enums/E_MovementSpeed Enum" :default "NewEnumerator0"))
  (returns (SpeedValue :type "Float (double-precision)"))
  (bind _output_get (set `CharacterMovementComponent.MaxWalkSpeed` (select `/Game/enemy/AI/Enums/E_MovementSpeed` Speed :`NewEnumerator1` 100.0 :`NewEnumerator2` 300.0 :`NewEnumerator3` 500.0 :!type "Float (single-precision)") (`self.CharacterMovement`)))
  (return _output_get))

(fn `UserConstructionScript`
  (`parent.UserConstructionScript`))