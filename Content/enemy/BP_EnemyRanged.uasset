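; Ranged enemy character that wields a crossbow, extending a parent enemy's startup and construction.
; BeginPlay spawns the crossbow onto the right-hand socket; Attack plays a rifle-fire montage whose notify makes noise and fires a BPCAttacks bullet trace at the AI controller's AttackTarget.
; Montage completion or interruption signals attack end.
; Accessor functions supply patrol route, ideal range and gait-based speed, and forward health and damage calls to BPCDamageSystem.
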(event `self.ReceiveBeginPlay`
  (`self.EquipWeapon`)
  (`parent.ReceiveBeginPlay`))

(event `/Game/enemy/AI/BPI_EnemyAI.EquipWeapon`
  (bind _returnvalue (`|SpawnActorFromClass` "/Game/weapons/blueprints/BP_WeaponCrossbow.BP_WeaponCrossbow_C" (`self.GetTransform`) "Undefined" "MultiplyWithRoot" null null))
  (bind _output_get (set `self.WeaponActor` _returnvalue))
  (`self.K2_AttachToComponent` _output_get (`self.Mesh`) "hand_rSocket" "SnapToTarget" "SnapToTarget" "SnapToTarget" true)
  (set `self.is_weilding_weapon` true)
  (`self.On weapon equiped`))

(event `/Game/enemy/AI/BPI_EnemyAI.Attack`
  (bind _notifyname (`|PlayMontage` (`self.Mesh`) "/Game/Characters/Mannequins/Animations/RifleAnims/AM_rifleFire.AM_rifleFire")
    (:`OnCompleted`
      (`self.On attack end` :!label _label))
    (:`OnInterrupted`
      (goto _label))
    (:`OnNotifyBegin`
      (switch `name` _notifyname
        (:`Fire`
          (`self.MakeNoise` 1.0 self (`self.K2_GetActorLocation`))
          (bind _asaic_enemy_base (cast `/Game/enemy/AI/AIC_enemy_base` (`AIBlueprintHelperLibrary.GetAIController` self)))
          (bind _attack_target (`/Game/enemy/AI/AIC_enemy_base.Attack Target` _asaic_enemy_base)
            (:`then`
              (`/Game/Attacks/BPC_Attacks.FireBullet` (`self.BPC_Attacks`) (`self.K2_GetActorLocation` (`self.WeaponActor`)) (`self.K2_GetActorLocation` _attack_target) (make `/Game/DamageSystem/S_DamageInfo` 10.0 "NewEnumerator2" "NewEnumerator1")))
            (:`else`)))))))

(fn `GetCurrentHealth`
  (returns (CurrentHealth :type "Float (double-precision)"))
  (return (`/Game/DamageSystem/BPC_DamageSystem.health` (`self.BPC_DamageSystem`))))

(fn `GetIdealRange`
  (returns (attackRadius :type "Float (double-precision)") (defendRadius :type "Float (double-precision)"))
  (return 600.0 600.0))

(fn `GetMaxHealth`
  (returns (MaxHealth :type "Float (double-precision)"))
  (return (`/Game/DamageSystem/BPC_DamageSystem.maxHealth` (`self.BPC_DamageSystem`))))

(fn `GetPatrolRoute`
  (returns (PatrolRoute :type "/Game/enemy/AI/BP_patrol_route Object Reference"))
  (return (`self.patrolRoute`)))

(fn `Heal`
  (params (Amount :type "Float (double-precision)"))
  (returns (NewHealth :type "Float (double-precision)"))
  (bind _newhealth (`/Game/DamageSystem/BPC_DamageSystem.Heal` (`self.BPC_DamageSystem`) Amount))
  (return _newhealth))

(fn `IsDead`
  (returns (Dead :type Boolean))
  (return (`/Game/DamageSystem/BPC_DamageSystem.isDead` (`self.BPC_DamageSystem`))))

(fn `SetMovementSpeed`
  (params (Speed :type "/Game/enemy/AI/Enums/E_MovementSpeed Enum" :default "NewEnumerator0"))
  (returns (SpeedValue :type "Float (double-precision)"))
  (bind _output_get (set `CharacterMovementComponent.MaxWalkSpeed` (select `/Game/enemy/AI/Enums/E_MovementSpeed` Speed :`NewEnumerator1` 200.0 :`NewEnumerator2` 300.0 :`NewEnumerator3` 500.0 :!type "Float (single-precision)") (`self.CharacterMovement`)))
  (return _output_get))

(fn `TakeDamage`
  (params (DamageInfo :type "/Game/DamageSystem/S_DamageInfo Structure") (DamageCauser :type "Actor Object Reference"))
  (returns (WasDamaged :type Boolean))
  (bind _wasdamaged (`/Game/DamageSystem/BPC_DamageSystem.TakeDamage` (`self.BPC_DamageSystem`) DamageInfo null))
  (return _wasdamaged))

(fn `UserConstructionScript`
  (`parent.UserConstructionScript`))