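; BPC_DamageSystem is a component that manages health, healing, damage and death for its owner.
; TakeDamage uses the CanBeDamaged macro to route a DamageInfo hit to block, damage or ignore, based on death, invincibility and blocking state.
; Blocks broadcast OnBlock with parry eligibility; damage broadcasts OnDeath when lethal, otherwise OnDamageResponse when the target is interruptible or interruption is forced.
; Heal restores clamped health only while alive.
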(fn `Heal`
  (params (Amount :type "Float (double-precision)"))
  (returns (NewHealth :type "Float (double-precision)"))
  (if (not (`self.isDead`))
    (bind _output_get (set `self.health` (`KismetMathLibrary.FClamp` (+ Amount (`self.health`)) 0.0 (`self.maxHealth`))))
    (return _output_get)))

(fn `TakeDamage`
  (params (DamageInfo :type "/Game/DamageSystem/S_DamageInfo Structure") (DamageSource :type "Actor Object Reference"))
  (returns (WasDamaged :type Boolean))
  (bind (_amount _damagetype _damageresponse _shoulddamageinvincible _canbeblocked _canbeparried _shouldforceinterrupt) (break `/Game/DamageSystem/S_DamageInfo` DamageInfo))
  (`self.CanBeDamaged` _shoulddamageinvincible _canbeblocked
    (:`BlockDamage`
      (`self.OnBlock` _canbeparried)
      (return false))
    (:`DoDamage`
      (bind _output_get (set `self.health` (- (`self.health`) _amount)))
      (bind _output_get_2 (set `self.isDead` (<= _output_get 0.0)))
      (if _output_get_2
        (`self.OnDeath` DamageSource)
        (elif (or _shouldforceinterrupt (`self.isInterruptible`))
          (`self.OnDamageResponse` _damageresponse DamageSource)))
      (return true))
    (:`NoDamage`
      (return false))))